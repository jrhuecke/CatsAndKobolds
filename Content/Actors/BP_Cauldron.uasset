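; Cauldron actor that brews potions over time and ejects each finished one as a world pickup.
; CreatePotion queues a potion's data asset with its brew time and adds a timer to the cauldron's widget-component UI.
; Tick counts down every queued brew and updates its timer, removing both when time runs out.
; Only the authority spawns the finished pickup, launching it upward with a randomized horizontal impulse.
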(event EventBeginPlay
  ;[1 1 1] Setting Timer UI
  (bind _asw_cauldron_ui (Utilities|Casting|CastToW_CauldronUI (UserInterface|GetUserWidgetObject (Variables|Default|GetBrewingTimers))))
  (Variables|Default|SetCauldronUI _asw_cauldron_ui))

(event EventTick
  (params (DeltaSeconds :type Float%20%28single-precision%29))
  (CallFunction|DecrementBrewingTimers))

(fn ConstructionScript)

(fn LaunchPotion
  (params (Potion%20Data%20Asset :type Potion%20Data%20Asset%20Blueprint%20Object%20Reference))
  (bind _tempforce (Variables|Default|GetTempForce))
  (bind _returnvalue (* _tempforce -1.0))
  (bind _returnvalue_2 (Game|SpawnActorfromClass "/Game/Actors/PotionWorldPickup.PotionWorldPickup_C" (Math|Transform|MakeTransform (+ (Transformation|GetActorLocation) (* (Transformation|GetActorUpVector) 100)) "0, 0, 0" "1.000000,1.000000,1.000000") "AdjustIfPossibleButAlwaysSpawn" "MultiplyWithRoot" 0 Potion%20Data%20Asset 0))
  (Physics|AddImpulse (Variables|/Game/Actors/PotionWorldPickup.PotionWorldPickup_C|GetPotion%20Mesh _returnvalue_2) (Math|Vector|MakeVector (Math|Random|RandomFloatinRange _returnvalue _tempforce) (Math|Random|RandomFloatinRange _returnvalue _tempforce) _tempforce) "None" true)
  (Development|PrintString "LaunchPotion"))

(fn DecrementBrewingTimers
  (for (_array_element _array_index) (Variables|Default|GetBrewingPotions)
    (if (<= (.BrewingTime (Utilities|Struct|BreakBrewingData _array_element)) 0.0)
      (Utilities|FlowControl|Sequence
        (:then_0
          (Networking|SwitchHasAuthority
            (:Authority
              (CallFunction|LaunchPotion (.PotionDataAsset (Utilities|Struct|BreakBrewingData _array_element))))))
        (:then_1
          (Default|RemoveTimer (Variables|Default|GetCauldronUI) (.TimerUI (Utilities|Struct|BreakBrewingData _array_element)))
          (Utilities|Array|RemoveIndex (Variables|Default|GetBrewingPotions) _array_index)))
      (else
        (Default|UpdateTimer (.TimerUI (Utilities|Struct|BreakBrewingData _array_element)) (Math|Float|Clamp(Float) (- (.BrewingTime (Utilities|Struct|BreakBrewingData _array_element)) (Utilities|Time|GetWorldDeltaSeconds)) 0.0 1e+02))
        (bind _structout (Utilities|Struct|SetmembersinBrewingData _array_element (Math|Float|Clamp(Float) (- (.BrewingTime (Utilities|Struct|BreakBrewingData _array_element)) (Utilities|Time|GetWorldDeltaSeconds)) 0.0 1e+02)))
        (Utilities|Array|SetArrayElem (Variables|Default|GetBrewingPotions) _array_index _structout)))))

(fn CreatePotion
  (params (Potion%20Data%20Asset :type Potion%20Data%20Asset%20Blueprint%20Object%20Reference))
  (bind _brewing_time (Variables|/Game/CoreBlueprints/PotionDataAssetBlueprint.PotionDataAssetBlueprint_C|GetBrewing%20Time Potion%20Data%20Asset))
  (bind _timerui (Default|AddTimer (Variables|Default|GetCauldronUI) Potion%20Data%20Asset))
  (Default|UpdateTimer _timerui _brewing_time)
  (Utilities|Array|Insert (Variables|Default|GetBrewingPotions) (Utilities|Struct|MakeBrewingData _brewing_time Potion%20Data%20Asset _timerui))
  (Development|PrintString "Started Brewing"))